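; Store actor that automatically sells a player's inventory when the character walks into its trigger box.
; On overlap, it casts to ThirdPersonCharacter and loops through the inventory items, adding each price to CurrentMoney and removing the item and its UI slot by index.
; Each sale and the new balance print to screen as debug text.
; Items are removed from the same array while it is being iterated.
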(event `self.Box.OnComponentBeginOverlap`
  (params (OverlappedComponent :type "PrimitiveComponent Object Reference") (OtherActor :type "Actor Object Reference") (OtherComp :type "PrimitiveComponent Object Reference") (OtherBodyIndex :type Integer) (bFromSweep :type Boolean) (SweepResult :type "HitResult Structure (by ref)"))
  (bind _asthird_person_character (cast `/Game/ThirdPersonBP/Blueprints/ThirdPersonCharacter` OtherActor))
  (bind _inventory (`/Game/ThirdPersonBP/Blueprints/ThirdPersonCharacter.Inventory` _asthird_person_character))
  (bind _items (`/Game/Blueprints/Inventory/Inventory.Items` _inventory))
  (for (_array_element _array_index) _items
    (bind (_name _price) (break `/Game/Blueprints/Inventory/Item` _array_element))
    (`KismetSystemLibrary.PrintString` (`KismetStringLibrary.Concat_StrStr` "Sold: " (`KismetTextLibrary.Conv_TextToString` _name)) true true (struct :`G` 1.0 :`B` 0.000716 :`A` 1.0) 5.0)
    (`KismetArrayLibrary.Array_RemoveItem` _items _array_element)
    (bind _output_get (set `/Game/Blueprints/Inventory/Inventory.Current Money` (+ (`/Game/Blueprints/Inventory/Inventory.Current Money` _inventory) _price) _inventory))
    (`/Game/Blueprints/Inventory/InventoryWidget.RemoveItemSlot` (`/Game/Blueprints/Inventory/Inventory.Inventory` _inventory) _array_index)
    (`KismetSystemLibrary.PrintString` (`KismetStringLibrary.Conv_DoubleToString` _output_get))))

(fn `UserConstructionScript`
  (`parent.UserConstructionScript`))